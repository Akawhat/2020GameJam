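; BP_Legs is a pickup that upgrades the ThirdPersonCharacter to a body with legs on overlap.
; It only acts when the character's CurrentState is 2, then swaps the mesh to Jogging, destroys itself and advances the state to 3.
; It also re-orients the mesh using the actor's forward vector, resizes the capsule half height and switches the animation class to FullBody_AnimBP.
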(event `self.ReceiveActorBeginOverlap`
  (params (OtherActor :type "Actor Object Reference"))
  (bind _asthird_person_character (cast `/Game/ThirdPersonBP/Blueprints/ThirdPersonCharacter` OtherActor))
  (if (== (`/Game/ThirdPersonBP/Blueprints/ThirdPersonCharacter.currentState` _asthird_person_character) 2)
    (bind _mesh (`Character.Mesh` _asthird_person_character))
    (`SkinnedMeshComponent.SetSkinnedAssetAndUpdate` _mesh "/Game/Models/FullBody/Jogging.Jogging" false)
    (`self.K2_DestroyActor`)
    (set `/Game/ThirdPersonBP/Blueprints/ThirdPersonCharacter.currentState` 3 _asthird_person_character)
    (bind (_returnvalue_roll _returnvalue_pitch _returnvalue_yaw) (`KismetMathLibrary.BreakRotator` (`KismetMathLibrary.MakeRotFromZ` (`self.GetActorForwardVector` _asthird_person_character))))
    (`SceneComponent.K2_SetWorldRotation` _mesh (`KismetMathLibrary.MakeRotator` 0.0 0.0 (+ _returnvalue_yaw 180.0)) false false)
    (`CapsuleComponent.SetCapsuleHalfHeight` (`Character.CapsuleComponent` _asthird_person_character) 55.0 true)
    (`SkeletalMeshComponent.SetAnimInstanceClass` (`Character.Mesh` _asthird_person_character) "/Game/Models/FullBody/FullBody_AnimBP.FullBody_AnimBP_C")))

(fn `UserConstructionScript`)